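; Base weapon pickup that gives a weapon to the player when a GunSystemCharacter overlaps it, then destroys itself.
; The construction script previews the weapon by spawning WeaponInfo's ViewWeapon class as a child actor and passing it that info.
; On overlap, WeaponInfo instantiates a new weapon, which is added to player 0's WeaponContainer regardless of which character triggered it.
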(event `self.ReceiveActorBeginOverlap`
  (params (OtherActor :type "Actor Object Reference"))
  (cast `GunSystemCharacter` OtherActor)
  (bind _returnvalue (`WeaponInfo.InstantiateWeapon` (`self.WeaponInfo`) self))
  (set `self.WeaponInstance` _returnvalue)
  (`WeaponContainer.AddWeapon` (`GunSystemCharacter.WeaponContainer` (cast `GunSystemCharacter` (`GameplayStatics.GetPlayerCharacter` 0) :!pure true)) (`self.WeaponInstance`))
  (`self.K2_DestroyActor`))

(fn `InstantiateWeapon`
  (bind _returnvalue (`AddComponent|NODE_AddChildActorComponent-1` :`bManualAttachment` true :`RelativeTransform` (`self.GetTransform`)))
  (bind _output_get (set `self.Weapon` _returnvalue))
  (`ChildActorComponent.SetChildActorClass` _output_get (`WeaponInfo.ViewWeapon` (`self.WeaponInfo`)))
  (bind _asweapon (cast `Weapon` (`ChildActorComponent.ChildActor` (`self.Weapon`))))
  (bind _output_get_2 (set `self.WeaponInstance` _asweapon))
  (`Weapon.UpdateWeaponInfo` _output_get_2 (`self.WeaponInfo`)))

(fn `UserConstructionScript`
  (`self.InstantiateWeapon`))