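; BP_Zoom is a gun-system weapon module that zooms the first-person player's camera by changing its field of view.
; Zoom divides the current FOV by ZoomScale and UnZoom multiplies it back, both instantly and relative to the current value.
; A timer-driven Lerp for smooth zooming is left disconnected, so the start and final FOV values computed on BeginPlay have no effect.
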(event `self.ReceiveBeginPlay`
  (bind _asfirst_person_character (cast `/Game/FirstPersonCPP/Blueprints/FirstPersonCharacter` (`GameplayStatics.GetPlayerCharacter` 0)))
  (bind _output_get (set `self.StartScale` (`CameraComponent.FieldOfView` (`GunSystemCharacter.FirstPersonCameraComponent` _asfirst_person_character))))
  (set `self.FinalScale` (* _output_get (`self.ZoomScale`))))

(event `CustomEvent_0`
  (bind _output_get (set `self.ScaleTime` (+ (`self.ScaleTime`) (* (`self.ZoomSpeed`) (`GameplayStatics.GetWorldDeltaSeconds`))))))

(event `self.Zoom`
  (bind _asfirst_person_character (cast `/Game/FirstPersonCPP/Blueprints/FirstPersonCharacter` (`GameplayStatics.GetPlayerCharacter` 0)))
  (set `self.ScaleTime` 0.0)
  (bind _firstpersoncameracomponent (`GunSystemCharacter.FirstPersonCameraComponent` _asfirst_person_character))
  (`CameraComponent.SetFieldOfView` _firstpersoncameracomponent (/ (`CameraComponent.FieldOfView` _firstpersoncameracomponent) (`self.ZoomScale`))))

(event `CustomEvent_1`
  (bind _output_get (set `self.ScaleTime` (`KismetMathLibrary.FClamp` (+ (`self.ScaleTime`) (* (`self.ZoomSpeed`) (`GameplayStatics.GetWorldDeltaSeconds`))))))
  (if (> _output_get 1.0)
    _))

(event `self.UnZoom`
  (bind _asfirst_person_character (cast `/Game/FirstPersonCPP/Blueprints/FirstPersonCharacter` (`GameplayStatics.GetPlayerCharacter` 0)))
  (bind _firstpersoncameracomponent (`GunSystemCharacter.FirstPersonCameraComponent` _asfirst_person_character))
  (`CameraComponent.SetFieldOfView` _firstpersoncameracomponent (* (`CameraComponent.FieldOfView` _firstpersoncameracomponent) (`self.ZoomScale`))))