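; BP_Katana_2 is a katana weapon Blueprint in the gun system, built on a parent class that supplies the attack logic.
; Left mouse press and release call StartAttack and StopAttack directly on the weapon.
; StartAttack, AttackTick and StopAttack each call the parent version, then print a placeholder debug string.
; BeginPlay waits briefly and prints the ShootingComponent's display name, so the asset adds only input hooks and debug output.
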(event `Key|LeftMouseButton`
  (params (Key :type "Key Structure"))
  (:`Pressed`
    (`self.StartAttack`))
  (:`Released`
    (`self.StopAttack`)))

(event `self.ReceiveBeginPlay`
  (`KismetSystemLibrary.Delay` 0.2)
  (`KismetSystemLibrary.PrintString` (`KismetSystemLibrary.GetDisplayName` (`self.ShootingComponent`))))

(event `self.StartAttack`
  (`parent.StartAttack`)
  (`KismetSystemLibrary.PrintString` "AAAAAA"))

(event `self.AttackTick`
  (`parent.AttackTick`)
  (`KismetSystemLibrary.PrintString` "OOOOO"))

(event `self.StopAttack`
  (`parent.StopAttack`)
  (`KismetSystemLibrary.PrintString` "AOAOAOAOAOAOA"))

(fn `UserConstructionScript`
  (`parent.UserConstructionScript`))