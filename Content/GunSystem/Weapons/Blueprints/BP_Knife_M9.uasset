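; BP_Knife_M9 is the M9 knife weapon Blueprint in the gun system, a child class that inherits its attack behavior from its parent.
; Its start, tick and stop attack events each call the parent and then print a placeholder debug string.
; On BeginPlay it waits briefly, then prints the display name of its ShootingComponent, and the construction script only calls the parent.
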(event `self.ReceiveBeginPlay`
  (`KismetSystemLibrary.Delay` 0.2)
  (`KismetSystemLibrary.PrintString` (`KismetSystemLibrary.GetDisplayName` (`self.ShootingComponent`))))

(event `self.StartAttack`
  (`parent.StartAttack`)
  (`KismetSystemLibrary.PrintString` "AAAAAA"))

(event `self.AttackTick`
  (`parent.AttackTick`)
  (`KismetSystemLibrary.PrintString` "OOOOO"))

(event `self.StopAttack`
  (`parent.StopAttack`)
  (`KismetSystemLibrary.PrintString` "AOAOAOAOAOAOA"))

(fn `UserConstructionScript`
  (`parent.UserConstructionScript`))