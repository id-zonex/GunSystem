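; AK-47 weapon Blueprint in the gun system that extends a parent weapon class.
; It overrides start attack, shoot, stop attack and weapon-info setup, passing each to the parent implementation.
; The added logic is debug printing only: the shooting component's name shortly after BeginPlay, placeholder text when attacks start and stop, and the name of each shot hit result entry.
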(event `self.ReceiveBeginPlay`
  (`KismetSystemLibrary.Delay` 0.2)
  (`KismetSystemLibrary.PrintString` (`KismetSystemLibrary.GetDisplayName` (`self.ShootingComponent`))))

(event `self.StartAttack`
  (`parent.StartAttack`)
  (`KismetSystemLibrary.PrintString` "Hello"))

(event `self.Shoot`
  (params (HitResult :type "Array of Actor Object Reference (by ref)"))
  (`parent.Shoot` HitResult)
  (for _array_element HitResult
    (`KismetSystemLibrary.PrintString` (`KismetSystemLibrary.GetDisplayName` _array_element))))

(event `self.StopAttack`
  (`parent.StopAttack`)
  (`KismetSystemLibrary.PrintString` "AOAOAOAOAOAOA"))

(event `self.ImplementWeaponInfo`
  (params (NewWeaponInfo :type "WeaponInfo Object Reference"))
  (`parent.ImplementWeaponInfo` NewWeaponInfo))

(fn `UserConstructionScript`
  (`parent.UserConstructionScript`))